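; GM_StealthKit is the stealth kit game mode that tracks level objectives and unlocks the end-of-level actors.
; Shortly after BeginPlay it counts actors carrying the objective tag and resets the taken count.
; End-level actors register themselves through AddEndLevel.
; CheckObjectives compares taken to total objectives and, when equal, unhides and activates every registered end-level actor.
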(event Custom|Check%20Objectives
  ;[1 1 1] If all objectives are taken, activates the end of level objectives
  (if (== (Variables|Default|GetNbObjectives) (Variables|Default|GetObjectivesTaken))
    (for _array_element (Variables|Default|GetEndLevelActors)
      (Rendering|SetActorHiddenInGame _array_element false)
      (Variables|/Game/GameKit/LevelRelated/EndLevelActor.EndLevelActor_C|SetisActive _array_element true))))

(event Custom|AddEndLevel
  (params (EndLevel :type End%20Level%20Actor%20Object%20Reference))
  ;[1 1 1] Creates a list of end of level objectives
  (Utilities|Array|Add (Variables|Default|GetEndLevelActors) EndLevel))

(event EventBeginPlay
  ;[1 1 1] Caclulate the number of objectives on the map
  (Utilities|FlowControl|Delay 0.2)
  (Variables|Default|SetNbObjectives 0)
  (Variables|Default|SetObjectivesTaken 0)
  (bind _outactors (Actor|GetAllActorswithTag (Variables|Default|GetTagObjective)))
  (for _array_element _outactors
    (Math|Integer|IncrementInt (Variables|Default|GetNbObjectives))))

(fn ConstructionScript)