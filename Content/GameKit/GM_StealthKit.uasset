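; Game mode for a stealth kit that tracks level objectives and detects the win condition.
; Shortly after BeginPlay, it resets both counters, counts the actors carrying the objective tag and prints the total.
; A CheckObjectives event compares that total with the taken count, which is not incremented in this graph, and prints a win message when they match.
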(event Custom|Check%20Objectives
  (if (== (Variables|Default|GetNbObjectives) (Variables|Default|GetObjectivesTaken))
    (Development|PrintString "Win")))

(event EventBeginPlay
  (Utilities|FlowControl|Delay 0.2)
  (Variables|Default|SetNbObjectives 0)
  (Variables|Default|SetObjectivesTaken 0)
  (bind _outactors (Actor|GetAllActorswithTag (Variables|Default|GetTagObjective)))
  (for _array_element _outactors
    (Math|Integer|IncrementInt (Variables|Default|GetNbObjectives)))
  (Development|PrintString (Utilities|String|ToString(Integer) (Variables|Default|GetNbObjectives))))

(fn ConstructionScript)